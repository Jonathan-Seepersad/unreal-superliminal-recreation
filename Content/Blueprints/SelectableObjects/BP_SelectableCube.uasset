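; BP_SelectableCube is a cube actor that can be selected through its BACSelectableComponent.
; On BeginPlay it binds the component's selected, deselected and moved callbacks, then sets a box trace method sized to half the Cube's local bounds extent, with zero orientation.
; Selection and deselection print the actor's display name for debugging, while the moved handler is empty.
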(event `self.ReceiveBeginPlay`
  (bind _bac_selectablecomponent (`self.BAC_SelectableComponent`))
  (bind (_min _max) (`StaticMeshComponent.GetLocalBounds` (`self.Cube`)))
  (add `/Game/Blueprints/SelectableObjects/BAC_SelectableComponent.On Selected` _bac_selectablecomponent (delegate `Actor Selected`))
  (add `/Game/Blueprints/SelectableObjects/BAC_SelectableComponent.On Deselected` _bac_selectablecomponent (delegate `Actor Deselected`))
  (add `/Game/Blueprints/SelectableObjects/BAC_SelectableComponent.On Object Moved` _bac_selectablecomponent (delegate `Object Moved`))
  (`/Game/Blueprints/SelectableObjects/BAC_SelectableComponent.Set Trace Method Box` :`self` _bac_selectablecomponent :`Half Size` (/ (- _max _min) (2.0 2.0 2.0))))

(event `Actor Selected`
  (`KismetSystemLibrary.PrintString` (`KismetStringLibrary.Concat_StrStr` "Selected: {" (`KismetSystemLibrary.GetDisplayName` null) "}")))

(event `Actor Deselected`
  (`KismetSystemLibrary.PrintString` (`KismetStringLibrary.Concat_StrStr` "Deselected: {" (`KismetSystemLibrary.GetDisplayName` null) "}")))

(event `Object Moved`)

(fn `UserConstructionScript`)