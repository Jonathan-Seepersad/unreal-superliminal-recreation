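; Selectable-object component that tracks selection, toggles the owner's primitive physics and collision, and moves and rescales it by forced perspective.
; DoTrace positions the primitive relative to a start transform, then box-traces toward it in interpolated segments.
; Each segment's box grows with distance; on a hit the object snaps there, scaled proportionally to preserve apparent size.
; Only box tracing is implemented, with debug drawing throughout; sphere and capsule are incomplete.
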(event `self.ReceiveBeginPlay`
  (bind _returnvalue (`Actor.GetComponentByClass` (`self.GetOwner`) "/Script/Engine.PrimitiveComponent"))
  (`/Engine/EditorBlueprintResources/StandardMacros.IsValid` (`self.Physics Primitive Component`)
    (:`Is Not Valid`
      (`/Engine/EditorBlueprintResources/StandardMacros.IsValid` _returnvalue
        (:`Is Valid`
          (`self.Set Physics Primitive Component` _returnvalue))
        (:`Is Not Valid`
          (`KismetSystemLibrary.PrintString` "Unable to pick Primitive component"))))))

(event `Set Physics Primitive Component`
  (params (Component :type "PrimitiveComponent Object Reference"))
  (set `self.Physics Primitive Component` Component))

(event `Set  Physics`
  (params (`Enabled?` :type Boolean))
  (bind _physics_primitive_component (`self.Physics Primitive Component`))
  (`PrimitiveComponent.SetSimulatePhysics` _physics_primitive_component `Enabled?`)
  (if `Enabled?`
    (`PrimitiveComponent.SetCollisionEnabled` _physics_primitive_component "QueryAndPhysics")
    (else
      (`PrimitiveComponent.SetCollisionEnabled` _physics_primitive_component "NoCollision"))))

(event `Selected`
  (set `self.Is Selected` true)
  (`self.On Selected`))

(event `self.ReceiveEndPlay`
  (params (EndPlayReason :type "EEndPlayReason Enum" :default "Destroyed"))
  (if (`self.Is Selected`)
    (`self.Deselected`)))

(event `Deselected`
  (set `self.Is Selected` false)
  (`self.On Deselected`))

(event `self.ReceiveTick`
  (params (DeltaSeconds :type "Float (single-precision)"))
  (`self.Draw Debug Shape` (struct :`R` 1.0 :`B` 1.0 :`A` 1.0)))

(event `Set Trace Method Box`
  (params (`Half Size` :type "Vector Structure") (Orientation :type "Rotator Structure"))
  (set `self.Shape Trace Method` "NewEnumerator0")
  (set `self.Box Half Size` `Half Size`)
  (set `self.Box Orientation` Orientation))

(event `Set Trace Method Sphere`
  (params (Radius :type "Float (double-precision)"))
  (set `self.Shape Trace Method` "NewEnumerator1")
  (set `self.Radius` Radius))

(event `Set Trace Method Capsule`
  (params (Radius :type "Float (double-precision)") (`Half Height` :type "Float (double-precision)"))
  (set `self.Shape Trace Method` "NewEnumerator2"))

(fn `Calculate New Scale`
  (params (`Current Start Point` :type "Vector Structure") (`Current End Point` :type "Vector Structure") (`Initial Distance` :type "Float (double-precision)") (`Old Scale` :type "Vector Structure"))
  (returns (`New Scale` :type "Vector Structure"))
  (return (* (/ (`KismetMathLibrary.Vector_Distance` `Current Start Point` `Current End Point`) `Initial Distance`) `Old Scale`)))

(fn `Do Trace`
  (params (`Start Transform` :type "Transform Structure") (`Initial Grab Transform` :type "Transform Structure") (`Trace Distance` :type "Float (double-precision)") (`Draw Debug Type` :type "EDrawDebugTrace Enum" :default "None"))
  (locals (`Primitive Original Transformation` :type "Transform Structure") (`Forward Vector` :type "Vector Structure" :default (0.0 0.0 0.0)) (`End Point` :type "Vector Structure") (`Original Distance` :type "Float (double-precision)" :default 0.0) (`Ignored Actors` :type "Array of Actor Object Reference") (`New Scale` :type "Vector Structure") (`Start Point` :type "Vector Structure" :default (0.0 0.0 0.0)) (`Far Cast Interpolation Count` :type Integer :default 300) (`Sub Start Point` :type "Vector Structure" :default (0.0 0.0 0.0)) (`Sub End Point` :type "Vector Structure" :default (0.0 0.0 0.0)) (`View Transformation` :type "Transform Structure") (`Loop Success` :type Boolean))
  (bind _start_point (`local.Start Point`))
  (bind (_initial_grab_transform_location _initial_grab_transform_rotation _initial_grab_transform_scale) (`KismetMathLibrary.BreakTransform` (`local.Initial Grab Transform`)))
  (bind _end_point (`local.End Point`))
  (bind _sub_end_point (`local.Sub End Point`))
  (bind (_initial_grab_transform_location_2 _initial_grab_transform_rotation_2 _initial_grab_transform_scale_2) (`KismetMathLibrary.BreakTransform` (`local.Initial Grab Transform`)))
  (bind _start_point_2 (`local.Start Point`))
  (bind _view_transformation_location (`KismetMathLibrary.BreakTransform` (`local.View Transformation`)))
  (bind _physics_primitive_component (`self.Physics Primitive Component`))
  (bind (_center _extent _rotation) (`self.Get Box at Scale` (`self.Calculate New Scale` (`local.Start Point`) _sub_end_point (`local.Original Distance`) _initial_grab_transform_scale)))
  (set `local.Start Point` `Start Transform_Location`)
  (bind _output_get (set `local.View Transformation` (`KismetMathLibrary.ComposeTransforms` `Initial Grab Transform` (`local.Start Transform`))))
  (`SceneComponent.K2_SetWorldTransform` (`self.Physics Primitive Component`) _output_get false false)
  (set `local.Original Distance` (`KismetMathLibrary.Vector_Distance` _view_transformation_location (`local.Start Point`)))
  (set `local.Ignored Actors` (`|MakeArray` (`self.GetOwner`)))
  (set `local.End Point` (+ _start_point_2 (* (`KismetMathLibrary.Normal` (- (`self.Get Box`) _start_point_2)) (`local.Trace Distance`))))
  (switch `/Game/Blueprints/SelectableObjects/BPE_TraceMethod` (`self.Shape Trace Method`)
    (:`NewEnumerator0`
      (for _index (range (+ (- (`local.Far Cast Interpolation Count`) 0) 1))
        (set `local.Sub Start Point` (`KismetMathLibrary.VLerp` _start_point _end_point (/ _index (`local.Far Cast Interpolation Count`))))
        (set `local.Sub End Point` (`KismetMathLibrary.VLerp` _start_point _end_point (/ (+ _index 1) (`local.Far Cast Interpolation Count`))))
        (bind (_outhit _returnvalue) (`KismetSystemLibrary.BoxTraceSingle` (`local.Sub Start Point`) _sub_end_point _extent _rotation "TraceTypeQuery1" false (`local.Ignored Actors`) "ForOneFrame" true (struct :`R` 1.0 :`G` 0.575142 :`A` 1.0) (struct :`R` 0.934119 :`G` 1.0 :`B` 0.979758 :`A` 1.0) 0.5))
        (`KismetSystemLibrary.DrawDebugSphere` (`local.Sub Start Point`) 5.0 12 (struct :`R` 1.0 :`G` 1.0 :`A` 1.0))
        (if _returnvalue
          (set `local.Loop Success` _returnvalue)
          (`KismetSystemLibrary.PrintString` "true")
          (break)
          (elif (== _index (`local.Far Cast Interpolation Count`))
            (`KismetSystemLibrary.PrintString` "False"))))
      (if (`local.Loop Success`)
        (`SceneComponent.K2_SetWorldLocation` _physics_primitive_component (`.Location` (`GameplayStatics.BreakHitResult` _outhit)) false false)
        (bind _new_scale (`self.Calculate New Scale` (`local.Start Point`) (`.Location` (`GameplayStatics.BreakHitResult` _outhit)) (`local.Original Distance`) _initial_grab_transform_scale_2))
        (`SceneComponent.SetWorldScale3D` _physics_primitive_component _new_scale)
        (bind (_center_2 _extent_2 _rotation_2) (`self.Get Box at Scale` _new_scale))
        (`KismetSystemLibrary.DrawDebugBox` _center_2 _extent_2 (struct :`R` 0.416448 :`G` 1.0 :`A` 1.0) _rotation_2)
        (else
          (return))))
    (:`NewEnumerator1`)
    (:`NewEnumerator2`)))

(fn `Draw Debug Shape`
  (params (`Line Color` :type "LinearColor Structure") (Duration :type "Float (double-precision)") (Thickness :type "Float (double-precision)"))
  (bind (_center _extent _rotation) (`self.Get Box`))
  (switch `/Game/Blueprints/SelectableObjects/BPE_TraceMethod` (`self.Shape Trace Method`)
    (:`NewEnumerator0`
      (`KismetSystemLibrary.DrawDebugBox` _center _extent (`local.Line Color`) _rotation))
    (:`NewEnumerator1`
      (`KismetSystemLibrary.DrawDebugSphere` (0.0 0.0 0.0)))
    (:`NewEnumerator2`
      (`KismetSystemLibrary.DrawDebugCapsule` (0.0 0.0 0.0)))))

(fn `Get Box`
  (returns (Center :type "Vector Structure") (Extent :type "Vector Structure") (Rotation :type "Rotator Structure"))
  (bind (_center _extent _rotation) (`self.Get Box at Scale` (`SceneComponent.K2_GetComponentScale` (`self.Physics Primitive Component`))))
  (return _center _extent _rotation))

(fn `Get Box at Scale`
  (params (Scale :type "Vector Structure"))
  (returns (Center :type "Vector Structure") (Extent :type "Vector Structure") (Rotation :type "Rotator Structure"))
  (bind (_returnvalue_location _returnvalue_rotation) (`KismetMathLibrary.BreakTransform` (`SceneComponent.K2_GetComponentToWorld` (`self.Physics Primitive Component`))))
  (return _returnvalue_location (* Scale (`self.Box Half Size`)) _returnvalue_rotation))

(fn `Is Selected?`
  (returns (Selected :type Boolean))
  (return (`self.Is Selected`)))